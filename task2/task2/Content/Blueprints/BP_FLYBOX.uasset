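; BP_FLYBOX is a flying target that players damage to score in a networked game.
; On the server, it picks a random world X/Y point at its current height every five seconds, and Tick eases the actor toward it with VInterpTo.
; Damage handled on the server increments the instigator's MyPlayerState score, asks MyGameMode to respawn a hit box, then destroys the actor.
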(event `self.ReceiveBeginPlay`
  (bind (_returnvalue_x _returnvalue_y _returnvalue_z) (`KismetMathLibrary.BreakVector` (`self.K2_GetActorLocation`)))
  (`/Engine/EditorBlueprintResources/ActorMacros.Switch Has Authority`
    (:`Authority`
      (set `self.AimPos` (`KismetMathLibrary.MakeVector` (`KismetMathLibrary.RandomFloatInRange` -400.0 400.0) (`KismetMathLibrary.RandomFloatInRange` -100.0 100.0) _returnvalue_z) :!label _label)
      (`KismetSystemLibrary.Delay` 5.0)
      (goto _label))))

(event `self.ReceiveTick`
  (params (DeltaSeconds :type "Float (single-precision)"))
  (`self.K2_SetActorLocation` (`KismetMathLibrary.VInterpTo` (`self.K2_GetActorLocation`) (`self.AimPos`) DeltaSeconds 1.0)))

(event `self.ReceiveAnyDamage`
  (params (Damage :type "Float (single-precision)") (DamageType :type "DamageType Object Reference") (InstigatedBy :type "Controller Object Reference") (DamageCauser :type "Actor Object Reference"))
  (`/Engine/EditorBlueprintResources/ActorMacros.Switch Has Authority`
    (:`Authority`
      (bind _asmy_player_state (cast `/Game/Blueprints/MyPlayerState` (`Controller.PlayerState` InstigatedBy)))
      (`/Game/Blueprints/MyPlayerState.IncrementScore` _asmy_player_state)
      (bind _asmy_game_mode (cast `/Game/Blueprints/MyGameMode` (`GameplayStatics.GetGameMode`)))
      (`/Game/Blueprints/MyGameMode.ReSpawnHitBox` _asmy_game_mode)
      (`self.K2_DestroyActor`))))

(fn `UserConstructionScript`)