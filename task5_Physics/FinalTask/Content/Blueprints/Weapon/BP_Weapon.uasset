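; BP_Weapon is a weapon pickup actor that the player collects by pressing F nearby.
; A sphere overlap with BP_MyCharacterOnly stores the character, allows pickup and enables input; any end overlap clears both reference and flag, leaving input enabled.
; F passes the weapon to the character's pickup function (捡取武器).
; The construction script writes the actor's own class into its WeaponInfo struct, keeping the other stats.
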(event `self.Sphere.OnComponentBeginOverlap`
  (params (OverlappedComponent :type "PrimitiveComponent Object Reference") (OtherActor :type "Actor Object Reference") (OtherComp :type "PrimitiveComponent Object Reference") (OtherBodyIndex :type Integer) (bFromSweep :type Boolean) (SweepResult :type "HitResult Structure (by ref)"))
  (bind _asbp_my_character_only (cast `/Game/MyCharacterBP/BP_MyCharacterOnly` OtherActor))
  (set `self.As My Character Only` _asbp_my_character_only)
  (set `self.CanPickUp?` true)
  (`self.EnableInput` (`GameplayStatics.GetPlayerController` 0)))

(event `self.Sphere.OnComponentEndOverlap`
  (params (OverlappedComponent :type "PrimitiveComponent Object Reference") (OtherActor :type "Actor Object Reference") (OtherComp :type "PrimitiveComponent Object Reference") (OtherBodyIndex :type Integer))
  (set `self.As My Character Only` null)
  (set `self.CanPickUp?` false))

(event `Key|F`
  (params (Key :type "Key Structure"))
  (bind _as_my_character_only (`self.As My Character Only`))
  (:`Pressed`
    (`/Engine/EditorBlueprintResources/StandardMacros.IsValid` _as_my_character_only
      (:`Is Valid`
        (if (`self.CanPickUp?`)
          (`/Game/MyCharacterBP/BP_MyCharacterOnly.捡取武器` _as_my_character_only self))))))

(fn `UserConstructionScript`
  (bind (_weapon_info_weapontype `_weapon_info_武器名称` _weapon_info_class `_weapon_info_图标` `_weapon_info_射击速度` `_weapon_info_开火声音` `_weapon_info_弹夹载弹量` `_weapon_info_当前装弹量` `_weapon_info_武器伤害值` _weapon_info_maxammo _weapon_info_weaponholdsocket _weapon_info_weaponequipsocket) (break `/Game/Blueprints/Weapon/S_WeaponInfo` (`self.Weapon_Info`)))
  (set `self.Weapon_Info` (make `/Game/Blueprints/Weapon/S_WeaponInfo` _weapon_info_weapontype `_weapon_info_武器名称` (`GameplayStatics.GetObjectClass` self) `_weapon_info_图标` `_weapon_info_射击速度` `_weapon_info_开火声音` `_weapon_info_弹夹载弹量` `_weapon_info_当前装弹量` `_weapon_info_武器伤害值` _weapon_info_maxammo _weapon_info_weaponholdsocket _weapon_info_weaponequipsocket)))