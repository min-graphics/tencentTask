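; MyGameState is a game state Blueprint with events for returning to the main menu and ending the game.
; The main menu event calls ShowMainMenuEvent on MyGameInstance.
; The game over event shows a QuitGame widget, switches player 0 to UI-only input and updates the game instance's CurrentState.
; The RepNotify functions for GameStartTimer and RandomTimerValue1 are empty.
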(event `返回主菜单`
  (bind _asmy_game_instance (cast `/Game/Blueprints/MyGameInstance` (`GameplayStatics.GetGameInstance`)))
  (`/Game/Blueprints/MyGameInstance.ShowMainMenuEvent` _asmy_game_instance))

(event `游戏结束`
  (bind _returnvalue (`GameplayStatics.GetPlayerController` 0))
  (bind _returnvalue_2 (`|CreateWidget` "/Game/Blueprints/Widgets/QuitGame.QuitGame_C" _returnvalue))
  (`UserWidget.AddToViewport` _returnvalue_2 0)
  (`WidgetBlueprintLibrary.SetInputMode_UIOnlyEx` _returnvalue _returnvalue_2)
  (bind _asmy_game_instance (cast `/Game/Blueprints/MyGameInstance` (`GameplayStatics.GetGameInstance`)))
  (set `/Game/Blueprints/MyGameInstance.CurrentState` "NewEnumerator8" _asmy_game_instance))

(fn `OnRep_GameStartTimer`)

(fn `OnRep_RandomTimerValue1`)

(fn `UserConstructionScript`)