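; BP_Grenade is a grenade actor that explodes on a fixed timer started at BeginPlay.
; When the timer fires, it spawns BP_Explosion at its transform, plays a 2D explosion sound and destroys itself.
; Static mesh hits cast the surface's physical material to FootPhycisc and play its sound in 2D, or print a placeholder debug string if the cast fails.
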(event `self.ReceiveBeginPlay`
  (`KismetSystemLibrary.K2_SetTimerDelegate` (delegate `Explosion`) 3.0))

(event `Explosion`
  (`|SpawnActorFromClass` "/Game/Blueprints/Weapon/BP_Explosion.BP_Explosion_C" (`self.GetTransform` self) "Undefined" "OverrideRootScale" null null)
  (`GameplayStatics.PlaySound2D` "/Game/Blueprints/Weapon/Explosion01.Explosion01" 1.0 1.0 0.0 null null)
  (`self.K2_DestroyActor`))

(event `self.StaticMesh.OnComponentHit`
  (params (HitComponent :type "PrimitiveComponent Object Reference") (OtherActor :type "Actor Object Reference") (OtherComp :type "PrimitiveComponent Object Reference") (NormalImpulse :type "Vector Structure") (Hit :type "HitResult Structure (by ref)"))
  (bind _asfoot_phycisc (cast `/Game/Materials/Phycisc/FootPhycisc` Hit_PhysMat)
    (:`then`
      (`GameplayStatics.PlaySound2D` (`/Game/Materials/Phycisc/FootPhycisc.Sound` _asfoot_phycisc) 1.0 1.0 0.0 null null))
    (:`CastFailed`
      (`KismetSystemLibrary.PrintString` "Hello"))))

(fn `UserConstructionScript`)